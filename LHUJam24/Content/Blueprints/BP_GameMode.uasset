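; BP_GameMode is a game mode Blueprint that runs the win condition as a survive-the-timer round.
; It binds to the StartGame and EndGameLose dispatchers on BeginPlay.
; Starting the game sets a timer for DayLength, and its expiry calls the EndGameWin dispatcher.
; A loss clears and invalidates that timer, so the win is not triggered.
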(event `self.ReceiveBeginPlay`
  (add `self.StartGame` (delegate `StartGame_Event`))
  (add `self.EndGame_Lose` (delegate `Event_Game_Lost`)))

(event `Event_Game_Lost`
  (`KismetSystemLibrary.K2_ClearAndInvalidateTimerHandle` (`self.Timer`)))

(event `StartGame_Event`
  (bind _returnvalue (`KismetSystemLibrary.K2_SetTimerDelegate` (delegate `TimerEnded`) (`self.DayLength`)))
  (set `self.Timer` _returnvalue))

(event `TimerEnded`
  (`self.EndGame_Win`))

(fn `UserConstructionScript`)